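; Tower stairs actor that can be activated and deactivated, toggling its collision and animating its material.
; The construction script creates a dynamic material instance on the mesh, and BeginPlay sets its "Level" parameter to -1 with collision off.
; Activate enables collision and plays a timeline that drives "Level", while Deactivate disables collision immediately and reverses the timeline.
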(event EventActivate
  (Collision|SetActorEnableCollision true)
  (bind _newtrack_0 (Timeline|Timeline_0 Play)
    (:Update
      (Rendering|Material|SetScalarParameterValue (Variables|Default|GetMat) "Level" _newtrack_0 :!class /Script/Engine.MaterialInstanceDynamic))))

(event EventDeactivate
  (Collision|SetActorEnableCollision false)
  (bind _newtrack_0 (Timeline|Timeline_0 Reverse)
    (:Update
      (Rendering|Material|SetScalarParameterValue (Variables|Default|GetMat) "Level" _newtrack_0 :!class /Script/Engine.MaterialInstanceDynamic))))

(event EventBeginPlay
  (Rendering|Material|SetScalarParameterValue (Variables|Default|GetMat) "Level" -1.0 :!class /Script/Engine.MaterialInstanceDynamic)
  (Collision|SetActorEnableCollision false))

(fn ConstructionScript
  (bind _returnvalue (Rendering|Material|CreateDynamicMaterialInstance (Variables|Default|GetMesh) 0 0 :!class /Script/Engine.PrimitiveComponent))
  (Variables|Default|SetMat _returnvalue))