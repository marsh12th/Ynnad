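; Light Vessel is a grabbable physics object that activates a Light_Emitter when dropped inside it, consuming itself.
; Overlap tracks the emitter, toggles Pawn collision and highlights the vessel if held over an inactive one.
; Timelines drive a dynamic material for highlight and spawn/consume fades, with overlaps ignored while fading.
; It registers in Capturer and player scene-capture show-only lists, storing indices for removal when consumed.
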(event OnComponentHit(Mesh)
  (params (HitComponent :type Primitive%20Component%20Object%20Reference) (OtherActor :type Actor%20Object%20Reference) (OtherComp :type Primitive%20Component%20Object%20Reference) (NormalImpulse :type Vector :default "0, 0, 0") (Hit :type Hit%20Result%20Structure%20%28by%20ref%29))
  ;[1 1 1] Enable gravity when hit
  (if (not (Class|PrimitiveComponent|IsGravityEnabled HitComponent))
    (Physics|SetEnableGravity (Variables|Default|GetMesh) true)))

(event OnComponentBeginOverlap(Mesh)
  (params (OverlappedComponent :type Primitive%20Component%20Object%20Reference) (OtherActor :type Actor%20Object%20Reference) (OtherComp :type Primitive%20Component%20Object%20Reference) (OtherBodyIndex :type Integer) (bFromSweep :type Boolean) (SweepResult :type Hit%20Result%20Structure%20%28by%20ref%29))
  ;[1 1 1] Checks if inside a vessel collector
  (if (not (Variables|Default|GetFading))
    (bind _aslight_emitter (Utilities|Casting|CastToLight_Emitter OtherActor))
    (Variables|Default|SetEmiiter_Within _aslight_emitter)
    (if (Variables|Default|GetGrabbed)
      (CallFunction|CheckHighlighting true)
      (Collision|SetCollisionResponsetoChannel (Variables|Default|GetMesh) "ECC_Pawn" "ECR_Block"))))

(event OnComponentEndOverlap(Mesh)
  (params (OverlappedComponent :type Primitive%20Component%20Object%20Reference) (OtherActor :type Actor%20Object%20Reference) (OtherComp :type Primitive%20Component%20Object%20Reference) (OtherBodyIndex :type Integer))
  ;[1 1 1] Checks if inside a vessel collector
  (if (not (Variables|Default|GetFading))
    (Utilities|Casting|CastToLight_Emitter OtherActor)
    (Variables|Default|SetEmiiter_Within 0)
    (CallFunction|CheckHighlighting false)
    (Collision|SetCollisionResponsetoChannel (Variables|Default|GetMesh) "ECC_Pawn" "ECR_Ignore")))

(event Custom|Drop
  (bind _emiiter_within (Variables|Default|GetEmiiter_Within))
  ;[1 1 1] Activate any emiiter if inside & consume vessel
  (Utilities|IsValid _emiiter_within
    (:Is%20Valid
      (if (and (not (Variables|/Game/Global/Blueprints/Light_Transport/Light_Emitter.Light_Emitter_C|GetIs_Active _emiiter_within)) (not (Variables|/Game/Global/Blueprints/Light_Transport/Light_Emitter.Light_Emitter_C|GetIs_Fading _emiiter_within)))
        (Default|Wake _emiiter_within)
        (Physics|SetEnableGravity (Variables|Default|GetMesh) false)
        (Variables|Default|SetFading true)
        (bind _fade (Timeline|Disappearing ReverseFromEnd)
          (:Update
            (Rendering|Material|SetVectorParameterValue (Variables|Default|GetMat) "Color" _fade :!class /Script/Engine.MaterialInstanceDynamic))
          (:Finished
            (Variables|Default|SetFading false)
            (Actor|DestroyActor)
            (CallFunction|RemovefromShownObjects)))))))

(event Custom|Check%20Highlighting
  (params (Entering :type Boolean))
  (bind _mat (Variables|Default|GetMat))
  ;[1 1 1] Color highlighting
  (if Entering
    (if (not (Variables|/Game/Global/Blueprints/Light_Transport/Light_Emitter.Light_Emitter_C|GetIs_Active (Variables|Default|GetEmiiter_Within)))
      (bind (_direction _emissionpower _color) (Timeline|Highlight Play)
        (:Update
          (Rendering|Material|SetVectorParameterValue _mat "Color" _color :!class /Script/Engine.MaterialInstanceDynamic)
          (Rendering|Material|SetScalarParameterValue _mat "Power" _emissionpower :!class /Script/Engine.MaterialInstanceDynamic))))
    (else
      (Timeline|Highlight Reverse))))

(event EventBeginPlay
  (CallFunction|AddtoShownObjects)
  ;[1 1 1] Start fade-in
  (Variables|Default|SetFading true)
  (bind _fade (Timeline|Appearing PlayFromStart)
    (:Update
      (Rendering|Material|SetVectorParameterValue (Variables|Default|GetMat) "Color" _fade :!class /Script/Engine.MaterialInstanceDynamic))
    (:Finished
      (Variables|Default|SetFading false))))

(fn ConstructionScript
  (bind _mesh (Variables|Default|GetMesh))
  (Collision|SetCollisionResponsetoChannel _mesh "ECC_Pawn" "ECR_Ignore")
  (bind _returnvalue (Rendering|Material|CreateDynamicMaterialInstance _mesh 0 0 :!class /Script/Engine.PrimitiveComponent))
  (Variables|Default|SetMat _returnvalue))

(fn AddtoShownObjects
  (bind _outactors (Actor|GetAllActorsOfClass "/Game/Global/Blueprints/Portals/Capturer.Capturer_C"))
  (bind _returnvalue (Utilities|Array|Add (Variables|/Script/Engine.SceneCaptureComponent|GetShowOnlyActors (Variables|/Script/Engine.SceneCapture2D|GetCaptureComponent2D (Utilities|Array|Get(acopy) _outactors))) self))
  (Variables|Default|SetCapturer_index _returnvalue)
  (bind _returnvalue_2 (Utilities|Array|Add (Variables|/Script/Engine.SceneCaptureComponent|GetShowOnlyActors (Variables|/Game/FirstPersonBP/FirstPersonCharacter.FirstPersonCharacter_C|GetPlayerCapturer (.AsFirst%20Person%20Character (Utilities|Casting|CastToFirstPersonCharacter (Game|Player|GetPlayerPawn 0))))) self))
  (Variables|Default|SetPlayerCam_index _returnvalue_2))

(fn RemovefromShownObjects
  (bind _outactors (Actor|GetAllActorsOfClass "/Game/Global/Blueprints/Portals/Capturer.Capturer_C"))
  (Utilities|Array|RemoveIndex (Variables|/Script/Engine.SceneCaptureComponent|GetShowOnlyActors (Variables|/Script/Engine.SceneCapture2D|GetCaptureComponent2D (Utilities|Array|Get(acopy) _outactors))) (Variables|Default|GetCapturer_index))
  (Utilities|Array|RemoveIndex (Variables|/Script/Engine.SceneCaptureComponent|GetShowOnlyActors (Variables|/Game/FirstPersonBP/FirstPersonCharacter.FirstPersonCharacter_C|GetPlayerCapturer (.AsFirst%20Person%20Character (Utilities|Casting|CastToFirstPersonCharacter (Game|Player|GetPlayerPawn 0))))) (Variables|Default|GetPlayerCam_index)))