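; Light emitter for the light-transport mechanic: a fire that can be collected, spawning a Light_Vessel, or woken to relight.
; Recolect and Wake swap fire and guide particles, crossfade sound and ramp light intensity by timeline, toggling the linked I_Activable partway through.
; IsFading blocks overlapping transitions; leaving the initial state swaps optional TextOut/TextIn prompts, and collection can destroy the emitter.
; The construction script derives starting visuals and audio from IsActive.
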(event Custom|Recolect
  (bind _text_out (Variables|Default|GetText_Out))
  (bind _text_in (Variables|Default|GetText_In))
  (bind _activable (Variables|Default|GetActivable))
  ;[1 1 1] Emitter desactivation
  (if (and (Variables|Default|GetIs_Active) (not (Variables|Default|GetIs_Fading)))
    (Variables|Default|SetIs_Fading true)
    (Utilities|FlowControl|Sequence
      (:then_0
        (if (Variables|Default|GetinitialState)
          (Utilities|FlowControl|Sequence
            (:then_0
              (Utilities|IsValid _text_out
                (:Is%20Valid
                  (Default|GoOut _text_out))))
            (:then_1
              (Utilities|IsValid _text_in
                (:Is%20Valid
                  (Default|Goin _text_in)))))))
      (:then_1
        ;;[1 1 1] Spawn vessel
        (Game|SpawnActorfromClass "/Game/Global/Blueprints/Light_Transport/Light_Vessel.Light_Vessel_C" (Transformation|GetActorTransform) "AdjustIfPossibleButAlwaysSpawn" 0 0)
        (Audio|PlaySoundatLocation "/Game/Sound/fire_out.fire_out" (Transformation|GetActorLocation))
        ;;[1 1 1] Shut down light emittes
        (Components|Activation|Deactivate (Variables|Default|GetFire_PS))
        (if (Variables|Default|GetDesroyOnDesactivation)
          _
          (else
            (Components|Activation|Activate (Variables|Default|GetGuide_PS) false)))
        (Audio|Components|Audio|FadeOut (Variables|Default|Getfire_sound) 2.0 0.0 :!class /Script/Engine.AudioComponent)
        (bind _fade_value (Timeline|Fade-out ReverseFromEnd)
          (:Update
            (Rendering|Components|Light|SetIntensity (Variables|Default|GetLight) (* (Variables|Default|GetLight_Intensity) _fade_value))
            (if (>= _fade_value 0.2)
              (Utilities|FlowControl|DoOnce false :!label _label
                (:Completed
                  (Utilities|IsValid _activable
                    (:Is%20Valid
                      (Default|Deactivate (.AsI%20Activable (Utilities|Casting|CastToI_Activable _activable)))))))))
          (:Finished
            (if (Variables|Default|GetDesroyOnDesactivation)
              (Actor|DestroyActor)
              (else
                (Variables|Default|SetIs_Active false)
                (Variables|Default|SetIs_Fading false)
                (goto _label Reset)))))))))

(event Custom|Wake
  (bind _activable (Variables|Default|GetActivable))
  (bind _text_out (Variables|Default|GetText_Out))
  (bind _text_in (Variables|Default|GetText_In))
  ;[1 1 1] Emitter activation
  (if (and (not (Variables|Default|GetIs_Active)) (not (Variables|Default|GetIs_Fading)))
    (Variables|Default|SetIs_Fading true)
    (Utilities|FlowControl|Sequence
      (:then_0
        (if (not (Variables|Default|GetinitialState))
          (Utilities|FlowControl|Sequence
            (:then_0
              (Utilities|IsValid _text_out
                (:Is%20Valid
                  (Default|GoOut _text_out))))
            (:then_1
              (Utilities|IsValid _text_in
                (:Is%20Valid
                  (Default|Goin _text_in)))))))
      (:then_1
        (Audio|PlaySound2D "/Game/Sound/vessel_out.vessel_out")
        ;;[1 1 1] Start again light emitters
        (Components|Activation|Activate (Variables|Default|GetFire_PS) false)
        (Components|Activation|Deactivate (Variables|Default|GetGuide_PS))
        (Audio|Components|Audio|FadeIn (Variables|Default|Getfire_sound) 3.0 1.0 0.0 :!class /Script/Engine.AudioComponent)
        (bind _fade_value (Timeline|Fade-in PlayFromStart)
          (:Update
            (Rendering|Components|Light|SetIntensity (Variables|Default|GetLight) (* (Variables|Default|GetLight_Intensity) _fade_value))
            (if (>= _fade_value 0.2)
              (Utilities|FlowControl|DoOnce false :!label _label
                (:Completed
                  (Utilities|IsValid _activable
                    (:Is%20Valid
                      (Default|Activate (.AsI%20Activable (Utilities|Casting|CastToI_Activable _activable)))))))))
          (:Finished
            (Variables|Default|SetIs_Active true)
            (Variables|Default|SetIs_Fading false)
            (goto _label Reset)))))))

(fn ConstructionScript
  (bind _is_active (Variables|Default|GetIs_Active))
  (Rendering|Components|Light|SetIntensity (Variables|Default|GetLight) (select (Variables|Default|GetIs_Active) (Variables|Default|GetLight_Intensity) 0.0))
  (Components|Activation|SetAutoActivate (Variables|Default|GetFire_PS) _is_active)
  (Components|Activation|SetAutoActivate (Variables|Default|GetGuide_PS) (not _is_active))
  (bind _output_get (Variables|Default|SetinitialState _is_active))
  (Components|Activation|SetAutoActivate (Variables|Default|Getfire_sound) _output_get))