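; Final cube actor for the Light Transport puzzle: a physics cube that spins up on BeginPlay and fades in and out as it is activated or deactivated.
; A Fade timeline drives the Level parameter of a dynamic material, while collision switches between query-and-physics and physics-only.
; PuzzleDone fades the cube out, sets Done to block further toggling, and calls DragDrop on the player's FirstPersonCharacter.
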(event Custom|Puzzle%20Done
  (CallFunction|Deactivate)
  (Variables|Default|SetDone true)
  (Default|Drag&Drop (.AsFirst%20Person%20Character (Utilities|Casting|CastToFirstPersonCharacter (Game|Player|GetPlayerPawn 0)))))

(event EventBeginPlay
  (Class|PrimitiveComponent|AddTorque (Variables|Default|GetCube) "50.000000,80.000000,120.000000" "None" true)
  (Rendering|Material|SetScalarParameterValue (Variables|Default|GetMat) "Level" 0.0 :!class /Script/Engine.MaterialInstanceDynamic))

(event EventActivate
  ;[1 1 1] Fade-in/-out
  (if (not (Variables|Default|GetDone))
    (Collision|SetCollisionEnabled (Variables|Default|GetCube) "QueryAndPhysics")
    (bind _value (Timeline|Fade Play)
      (:Update
        (Rendering|Material|SetScalarParameterValue (Variables|Default|GetMat) "Level" _value :!class /Script/Engine.MaterialInstanceDynamic)))))

(event EventDeactivate
  ;[1 1 1] Fade-in/-out
  (if (not (Variables|Default|GetDone))
    (Collision|SetCollisionEnabled (Variables|Default|GetCube) "PhysicsOnly")
    (bind _value (Timeline|Fade Reverse)
      (:Update
        (Rendering|Material|SetScalarParameterValue (Variables|Default|GetMat) "Level" _value :!class /Script/Engine.MaterialInstanceDynamic)))))

(fn ConstructionScript
  (bind _returnvalue (Rendering|Material|CreateDynamicMaterialInstance (Variables|Default|GetCube) 0 0 :!class /Script/Engine.PrimitiveComponent))
  (Variables|Default|SetMat _returnvalue))