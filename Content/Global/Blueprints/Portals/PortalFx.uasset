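; PortalFx is a set of portal math helpers that map directions, rotations and locations from a current portal to a target portal.
; Each converts into the current portal's local space, negates X and Y for a half turn, then transforms out through the target portal.
; Rotations are rebuilt from their converted X and Y axes.
; The player location variant uses the same math as the general location function.
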(fn PortalConvertDirection
  (params (Direction :type Vector) (Current%20Portal :type Portal%20Object%20Reference) (Target%20Portal :type Portal%20Object%20Reference))
  (return (Math|Transform|TransformDirection (Transformation|GetActorTransform Target%20Portal) (* (Math|Transform|InverseTransformDirection (Transformation|GetActorTransform Current%20Portal) Direction) "-1.000000,-1.000000,1.000000"))))

(fn PortalConvertRotator
  (params (Rotator :type Rotator) (Current%20Portal :type Portal%20Object%20Reference) (Target%20Portal :type Portal%20Object%20Reference))
  (bind (_x _y) (Math|Rotator|GetAxes Rotator))
  (bind _result_direction (CallFunction|PortalConvertDirection _x Current%20Portal Target%20Portal))
  (bind _result_direction_2 (CallFunction|PortalConvertDirection _y Current%20Portal Target%20Portal))
  (return (Math|Rotator|MakeRotfromXY _result_direction _result_direction_2)))

(fn PortalConvertLocation
  (params (Location :type Vector) (Current%20Portal :type Portal%20Object%20Reference) (Target%20Portal :type Portal%20Object%20Reference))
  (return (Math|Transform|TransformLocation (Transformation|GetActorTransform Target%20Portal) (* (Math|Transform|InverseTransformLocation (Transformation|GetActorTransform Current%20Portal) Location) "-1.000000,-1.000000,1.000000"))))

(fn PortalConvertLocationPlayer
  (params (Location :type Vector) (Current%20Portal :type Portal%20Object%20Reference) (Target%20Portal :type Portal%20Object%20Reference))
  (return (Math|Transform|TransformLocation (Transformation|GetActorTransform Target%20Portal) (* (Math|Transform|InverseTransformLocation (Transformation|GetActorTransform Current%20Portal) Location) "-1.000000,-1.000000,1.000000"))))