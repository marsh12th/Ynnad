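; Portal actor that teleports the first-person player to its linked target portal when hit while facing it from the front and falling.
; It drops any carried object, converts the player's location, turns the view 180 degrees and launches them out along the target's right vector with collision briefly disabled.
; It then switches the scene Capturer to the target portal and, if the puzzle is done, disables both portals and clears their surface stencil.
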(event Collision|EventHit
  (params (MyComp :type Primitive%20Component%20Object%20Reference) (Other :type Actor%20Object%20Reference) (OtherComp :type Primitive%20Component%20Object%20Reference) (bSelfMoved :type Boolean) (HitLocation :type Vector :default "0, 0, 0") (HitNormal :type Vector :default "0, 0, 0") (NormalImpulse :type Vector :default "0, 0, 0") (Hit :type Hit%20Result%20Structure%20%28by%20ref%29))
  (bind _targetportal (Variables|PortalConfig|GetTargetPortal))
  (if (not (Variables|Default|GetNotWorking))
    (bind _asfirst_person_character (Utilities|Casting|CastToFirstPersonCharacter Other))
    (if (and (and (<= (Utilities|AngleBetweenPlayer) 4e+01) (AI|Components|NavMovement|IsFalling (Variables|/Script/Engine.Character|GetCharacterMovement _asfirst_person_character))) (>= (.Y (Math|Vector|BreakVector (Math|Transform|InverseTransformLocation (Transformation|GetActorTransform) (Transformation|GetActorLocation _asfirst_person_character)))) 0.0))
      (Utilities|FlowControl|Sequence
        (:then_0
          ;[1 1 1] Can't carry objects through the portal
          (if (Variables|/Game/FirstPersonBP/FirstPersonCharacter.FirstPersonCharacter_C|GetIs_Grabbing _asfirst_person_character)
            (Default|Drag&Drop _asfirst_person_character)))
        (:then_1
          (Collision|SetActorEnableCollision _asfirst_person_character false)
          (CallFunction|TeleportPlayer _asfirst_person_character)
          (bind _outactors (Actor|GetAllActorsOfClass "/Game/Global/Blueprints/Portals/Capturer.Capturer_C"))
          (Default|ChangePortal (Utilities|Array|Get(acopy) _outactors) (Variables|PortalConfig|GetTargetPortal) (Variables|Default|GetWill_Show_Only_Objs))
          (if (Variables|Default|GetPuzzle_Done)
            (Rendering|SetCustomDepthStencilValue (Variables|Default|GetPortal_surface) 0)
            (Variables|Default|SetNotWorking true)
            (Variables|Portal_C|SetPuzzle_Done _targetportal true)
            (Variables|Portal_C|SetNotWorking _targetportal true)
            (Rendering|SetCustomDepthStencilValue (Variables|Portal_C|GetPortal_surface _targetportal) 0))
          (Utilities|FlowControl|Delay 0.3)
          (Collision|SetActorEnableCollision (.AsFirst%20Person%20Character (Utilities|Casting|CastToFirstPersonCharacter (Game|Player|GetPlayerPawn 0))) true))))))

(fn ConstructionScript)

(fn TeleportPlayer
  (params (Player :type First%20Person%20Character%20Object%20Reference))
  (bind _returnvalue (Pawn|GetController Player))
  (bind _self self)
  (bind _targetportal (Variables|PortalConfig|GetTargetPortal))
  (bind _result_location (CallFunction|PortalConvertLocationPlayer (Transformation|GetActorLocation Player) _self _targetportal))
  (LocalVariables|SetNewLocation _result_location)
  (bind _result_rotator (CallFunction|PortalConvertRotator (Transformation|GetActorRotation Player) _self _targetportal))
  (LocalVariables|SetNewRotator _result_rotator)
  (Transformation|SetActorLocation Player (LocalVariables|GetNewLocation) false false)
  (Pawn|SetControlRotation _returnvalue (Math|Rotator|CombineRotators (Pawn|GetControlRotation _returnvalue :!class /Script/Engine.Controller) "0,180.000000, 0"))
  (Variables|/Script/Engine.MovementComponent|SetVelocity (Variables|/Script/Engine.Character|GetCharacterMovement Player) (* (Transformation|GetActorRightVector (Variables|PortalConfig|GetTargetPortal)) 5e+02)))