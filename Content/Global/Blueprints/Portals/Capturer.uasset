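; Portal capturer actor that renders the view through the current portal from its linked target portal with a SceneCapture2D.
; Every tick it converts the player camera's transform between the two portals and sets a clip plane at the target's surface.
; ChangePortal switches the portal pair and show-only list, adding the player and handing the previous list to the player's PlayerCapturer.
; SoyUnPie only prints a debug string.
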(event Custom|SoyUnPie
  (Development|PrintString "HolaPIEEEEEEEEEEEEEE"))

(event Custom|Change%20Portal
  (params (NewCurrentPortal :type Portal%20Object%20Reference) (ShowOnlyObjs :type Array%20of%20Actor%20Object%20References))
  ;[1 1 1] Swaps portal came ras
  (CallFunction|ChangeShownOnlyObject ShowOnlyObjs)
  (bind _output_get (Variables|Default|SetCurrent_Portal NewCurrentPortal))
  (Variables|Default|SetTarget_Portal (Variables|/Game/Global/Blueprints/Portals/Portal.Portal_C|GetTargetPortal _output_get)))

(event EventTick
  (params (DeltaSeconds :type Float%20%28single-precision%29))
  (bind _player (Variables|Default|GetPlayer))
  (bind _target_portal (Variables|Default|GetTarget_Portal))
  (bind _current_portal (Variables|Default|GetCurrent_Portal))
  (bind _target_portal_2 (Variables|Default|GetTarget_Portal))
  (bind _firstpersoncamera (Variables|/Game/FirstPersonBP/FirstPersonCharacter.FirstPersonCharacter_C|GetFirstPersonCamera _player))
  ;[1 1 1] Capturer location & rotation
  (bind _result_location (CallFunction|PortalConvertLocation (Transformation|GetWorldLocation _firstpersoncamera) _current_portal _target_portal_2))
  (bind _result_rotator (CallFunction|PortalConvertRotator (Transformation|GetWorldRotation _firstpersoncamera) _current_portal _target_portal_2))
  (Transformation|SetActorLocationAndRotation _result_location _result_rotator)
  ;[1 1 1] Clipping planes
  (Variables|/Script/Engine.SceneCaptureComponent2D|SetClipPlaneBase (Variables|DecalActor|GetCaptureComponent2D) (Transformation|GetWorldLocation (Variables|/Game/Global/Blueprints/Portals/Portal.Portal_C|GetPortal_surface _target_portal)))
  (Variables|/Script/Engine.SceneCaptureComponent2D|SetClipPlaneNormal (Variables|DecalActor|GetCaptureComponent2D) (Transformation|GetActorRightVector _target_portal)))

(event EventBeginPlay
  ;[1 1 1] Var assign
  (Variables|Default|SetTarget_Portal (Variables|/Game/Global/Blueprints/Portals/Portal.Portal_C|GetTargetPortal (Variables|Default|GetCurrent_Portal)))
  (Variables|Default|SetPlayer (.AsFirst%20Person%20Character (Utilities|Casting|CastToFirstPersonCharacter (Game|GetPlayerCharacter 0)))))

(fn ConstructionScript)

(fn ChangeShownOnlyObject
  (params (Passed_Array :type Array%20of%20Actor%20Object%20References))
  (bind _returnvalue (Game|Player|GetPlayerPawn 0))
  (bind _capturecomponent2d (Variables|DecalActor|GetCaptureComponent2D))
  (bind _asfirst_person_character (Utilities|Casting|CastToFirstPersonCharacter _returnvalue))
  (Utilities|Array|Add Passed_Array _asfirst_person_character)
  (Utilities|Array|Add (Variables|/Script/Engine.SceneCaptureComponent|GetShowOnlyActors _capturecomponent2d) _asfirst_person_character)
  (Variables|/Script/Engine.SceneCaptureComponent|SetShowOnlyActors (Variables|/Game/FirstPersonBP/FirstPersonCharacter.FirstPersonCharacter_C|GetPlayerCapturer _asfirst_person_character) (Variables|/Script/Engine.SceneCaptureComponent|GetShowOnlyActors _capturecomponent2d))
  (Variables|/Script/Engine.SceneCaptureComponent|SetShowOnlyActors _capturecomponent2d Passed_Array))