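; Good_Text is a text actor that fades in and out once as the player walks through trigger volumes.
; The construction script creates a dynamic material, assigns the text texture and sets the fade timeline's length from Duration.
; Appear overlap or Go_In plays the timeline and Dissapear overlap or Go_Out reverses it, each behind a DoOnce.
; The timeline drives the material's Value parameter, which starts at zero.
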(event OnComponentBeginOverlap(Dissapear)
  (params (OverlappedComponent :type Primitive%20Component%20Object%20Reference) (OtherActor :type Actor%20Object%20Reference) (OtherComp :type Primitive%20Component%20Object%20Reference) (OtherBodyIndex :type Integer) (bFromSweep :type Boolean) (SweepResult :type Hit%20Result%20Structure%20%28by%20ref%29))
  (Utilities|Casting|CastToFirstPersonCharacter OtherActor)
  (Utilities|FlowControl|DoOnce false
    (:Completed
      (bind _fade_value (Timeline|Fading Reverse)
        (:Update
          (Rendering|Material|SetScalarParameterValue (Variables|Default|GetMat) "Value" _fade_value :!class /Script/Engine.MaterialInstanceDynamic))))))

(event OnComponentBeginOverlap(Appear)
  (params (OverlappedComponent :type Primitive%20Component%20Object%20Reference) (OtherActor :type Actor%20Object%20Reference) (OtherComp :type Primitive%20Component%20Object%20Reference) (OtherBodyIndex :type Integer) (bFromSweep :type Boolean) (SweepResult :type Hit%20Result%20Structure%20%28by%20ref%29))
  (Utilities|Casting|CastToFirstPersonCharacter OtherActor)
  (Utilities|FlowControl|DoOnce false
    (:Completed
      (bind _fade_value (Timeline|Fading Play)
        (:Update
          (Rendering|Material|SetScalarParameterValue (Variables|Default|GetMat) "Value" _fade_value :!class /Script/Engine.MaterialInstanceDynamic))))))

(event Custom|Go_Out
  (Utilities|FlowControl|DoOnce false
    (:Completed
      (bind _fade_value (Timeline|Fading Reverse)
        (:Update
          (Rendering|Material|SetScalarParameterValue (Variables|Default|GetMat) "Value" _fade_value :!class /Script/Engine.MaterialInstanceDynamic))))))

(event Custom|Go_In
  (Utilities|FlowControl|DoOnce false
    (:Completed
      (bind _fade_value (Timeline|Fading Play)
        (:Update
          (Rendering|Material|SetScalarParameterValue (Variables|Default|GetMat) "Value" _fade_value :!class /Script/Engine.MaterialInstanceDynamic))))))

(event EventBeginPlay
  (Rendering|Material|SetScalarParameterValue (Variables|Default|GetMat) "Value" 0.0 :!class /Script/Engine.MaterialInstanceDynamic))

(fn ConstructionScript
  (bind _returnvalue (Rendering|Material|CreateDynamicMaterialInstance (Variables|Default|GetText) 0 0 :!class /Script/Engine.PrimitiveComponent))
  (bind _output_get (Variables|Default|SetMat _returnvalue))
  (Rendering|Material|SetTextureParameterValue _output_get "Text" (Variables|Default|GetText_Texture))
  (Components|Timeline|SetTimelineLength (Variables|Default|GetFading) (Variables|Default|GetDuration)))